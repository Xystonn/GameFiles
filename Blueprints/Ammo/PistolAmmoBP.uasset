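; Pistol ammo pickup that tops up the first-person character's ammo when its box is overlapped, provided the pistol has been picked up.
; It adds 10 to the reserve, or fills magazine and reserve to the 50-round cap when the total is nearly full.
; It destroys itself only when ammo is granted.
; Tick spins the actor by a fixed step each frame, independent of delta time.
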(event `self.Box.OnComponentBeginOverlap`
  (params (OverlappedComponent :type "PrimitiveComponent Object Reference") (OtherActor :type "Actor Object Reference") (OtherComp :type "PrimitiveComponent Object Reference") (OtherBodyIndex :type Integer) (bFromSweep :type Boolean) (SweepResult :type "HitResult Structure (by ref)"))
  (bind _asfirst_person_character_bp (cast `/Game/FirstPersonBP/AllAssets/Blueprints/FirstPersonCharacterBP` OtherActor))
  (bind _haspistolbeenpickedup (`/Game/FirstPersonBP/AllAssets/Blueprints/FirstPersonCharacterBP.HasPistolBeenPickedUp` _asfirst_person_character_bp))
  (bind _totalpistolammo (`/Game/FirstPersonBP/AllAssets/Blueprints/FirstPersonCharacterBP.TotalPistolAmmo` _asfirst_person_character_bp))
  (bind _returnvalue (+ _totalpistolammo (`/Game/FirstPersonBP/AllAssets/Blueprints/FirstPersonCharacterBP.AmmoInPistolMag` _asfirst_person_character_bp)))
  (if (and _haspistolbeenpickedup (<= _returnvalue 40))
    (set `/Game/FirstPersonBP/AllAssets/Blueprints/FirstPersonCharacterBP.TotalPistolAmmo` (+ _totalpistolammo 10) _asfirst_person_character_bp)
    (`self.K2_DestroyActor` :!label _label)
    (elif (and _haspistolbeenpickedup (< _returnvalue 50))
      (set `/Game/FirstPersonBP/AllAssets/Blueprints/FirstPersonCharacterBP.AmmoInPistolMag` 10 _asfirst_person_character_bp)
      (set `/Game/FirstPersonBP/AllAssets/Blueprints/FirstPersonCharacterBP.TotalPistolAmmo` 40 _asfirst_person_character_bp)
      (goto _label))))

(event `self.ReceiveTick`
  (params (DeltaSeconds :type "Float (single-precision)"))
  (`self.K2_AddActorLocalRotation` (struct :`Yaw` 3.0)))

(fn `UserConstructionScript`)