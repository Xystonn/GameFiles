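; Machine gun ammo pickup that refills FirstPersonCharacterBP on box overlap, only once that character has picked up the machine gun.
; It adds a fixed amount to reserve ammo, or near the combined cap sets both magazine and reserve to full, then destroys itself.
; At full ammo it stays in the world.
; Tick spins it by a fixed step per frame, without delta-time scaling.
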(event `self.Box.OnComponentBeginOverlap`
  (params (OverlappedComponent :type "PrimitiveComponent Object Reference") (OtherActor :type "Actor Object Reference") (OtherComp :type "PrimitiveComponent Object Reference") (OtherBodyIndex :type Integer) (bFromSweep :type Boolean) (SweepResult :type "HitResult Structure (by ref)"))
  (bind _asfirst_person_character_bp (cast `/Game/FirstPersonBP/AllAssets/Blueprints/FirstPersonCharacterBP` OtherActor))
  (bind _totalmachinegunammo (`/Game/FirstPersonBP/AllAssets/Blueprints/FirstPersonCharacterBP.TotalMachineGunAmmo` _asfirst_person_character_bp))
  (bind _returnvalue (+ (`/Game/FirstPersonBP/AllAssets/Blueprints/FirstPersonCharacterBP.AmmoInMachineGunMag` _asfirst_person_character_bp) _totalmachinegunammo))
  (bind _hasmachinegunbeenpickedup (`/Game/FirstPersonBP/AllAssets/Blueprints/FirstPersonCharacterBP.HasMachineGunBeenPickedUp` _asfirst_person_character_bp))
  (if (and (<= _returnvalue 96) _hasmachinegunbeenpickedup)
    (set `/Game/FirstPersonBP/AllAssets/Blueprints/FirstPersonCharacterBP.TotalMachineGunAmmo` (+ _totalmachinegunammo 64) _asfirst_person_character_bp)
    (`self.K2_DestroyActor` :!label _label)
    (elif (and _hasmachinegunbeenpickedup (< _returnvalue 160))
      (set `/Game/FirstPersonBP/AllAssets/Blueprints/FirstPersonCharacterBP.TotalMachineGunAmmo` 80 _asfirst_person_character_bp)
      (set `/Game/FirstPersonBP/AllAssets/Blueprints/FirstPersonCharacterBP.AmmoInMachineGunMag` 80 _asfirst_person_character_bp)
      (goto _label))))

(event `self.ReceiveTick`
  (params (DeltaSeconds :type "Float (single-precision)"))
  (`self.K2_AddActorLocalRotation` (struct :`Yaw` 3.0)))

(fn `UserConstructionScript`)