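; Shotgun ammo pickup that spins a fixed step every tick, so its speed depends on frame rate.
; On box overlap by FirstPersonCharacterBP with the shotgun already picked up, it adds six shells to the reserve.
; Near the 42-shell combined cap, it instead fills both magazine and reserve to maximum.
; It destroys itself only when ammo is granted, otherwise staying in the world.
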(event `self.Box.OnComponentBeginOverlap`
  (params (OverlappedComponent :type "PrimitiveComponent Object Reference") (OtherActor :type "Actor Object Reference") (OtherComp :type "PrimitiveComponent Object Reference") (OtherBodyIndex :type Integer) (bFromSweep :type Boolean) (SweepResult :type "HitResult Structure (by ref)"))
  (bind _asfirst_person_character_bp (cast `/Game/FirstPersonBP/AllAssets/Blueprints/FirstPersonCharacterBP` OtherActor))
  (bind _hasshotgunbeenpickedup (`/Game/FirstPersonBP/AllAssets/Blueprints/FirstPersonCharacterBP.HasShotgunBeenPickedUp` _asfirst_person_character_bp))
  (bind _totalshotgunammo (`/Game/FirstPersonBP/AllAssets/Blueprints/FirstPersonCharacterBP.TotalShotgunAmmo` _asfirst_person_character_bp))
  (bind _returnvalue (+ _totalshotgunammo (`/Game/FirstPersonBP/AllAssets/Blueprints/FirstPersonCharacterBP.AmmoInShotgunMag` _asfirst_person_character_bp)))
  (if (and _hasshotgunbeenpickedup (<= _returnvalue 36))
    (set `/Game/FirstPersonBP/AllAssets/Blueprints/FirstPersonCharacterBP.TotalShotgunAmmo` (+ _totalshotgunammo 6) _asfirst_person_character_bp)
    (`self.K2_DestroyActor` :!label _label)
    (elif (and _hasshotgunbeenpickedup (< _returnvalue 42))
      (set `/Game/FirstPersonBP/AllAssets/Blueprints/FirstPersonCharacterBP.AmmoInShotgunMag` 6 _asfirst_person_character_bp)
      (set `/Game/FirstPersonBP/AllAssets/Blueprints/FirstPersonCharacterBP.TotalShotgunAmmo` 36 _asfirst_person_character_bp)
      (goto _label))))

(event `self.ReceiveTick`
  (params (DeltaSeconds :type "Float (single-precision)"))
  (`self.K2_AddActorLocalRotation` (struct :`Yaw` 3.0)))

(fn `UserConstructionScript`)