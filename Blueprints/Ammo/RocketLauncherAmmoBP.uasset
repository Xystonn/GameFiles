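; Rocket launcher ammo pickup that spins every tick and destroys itself when collected.
; On mesh overlap, a first-person character who has picked up the launcher gains reserve rockets while combined ammo is low.
; Just below the cap, it instead overwrites magazine and reserve with fixed full values; at the cap the pickup stays.
; The construction script also sets a Projectile component's initial speed from a variable.
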(event `self.StaticMesh.OnComponentBeginOverlap`
  (params (OverlappedComponent :type "PrimitiveComponent Object Reference") (OtherActor :type "Actor Object Reference") (OtherComp :type "PrimitiveComponent Object Reference") (OtherBodyIndex :type Integer) (bFromSweep :type Boolean) (SweepResult :type "HitResult Structure (by ref)"))
  (bind _asfirst_person_character_bp (cast `/Game/FirstPersonBP/AllAssets/Blueprints/FirstPersonCharacterBP` OtherActor))
  (bind _hasrocketlauncherbeenpickedup_ (`/Game/FirstPersonBP/AllAssets/Blueprints/FirstPersonCharacterBP.HasRocketLauncherBeenPickedUp?` _asfirst_person_character_bp))
  (bind _totalrocketlauncherammo (`/Game/FirstPersonBP/AllAssets/Blueprints/FirstPersonCharacterBP.TotalRocketLauncherAmmo` _asfirst_person_character_bp))
  (bind _returnvalue (+ _totalrocketlauncherammo (`/Game/FirstPersonBP/AllAssets/Blueprints/FirstPersonCharacterBP.AmmoInRocketLauncherMag` _asfirst_person_character_bp)))
  (if (and _hasrocketlauncherbeenpickedup_ (<= _returnvalue 4))
    (set `/Game/FirstPersonBP/AllAssets/Blueprints/FirstPersonCharacterBP.TotalRocketLauncherAmmo` (+ _totalrocketlauncherammo 2) _asfirst_person_character_bp)
    (`self.K2_DestroyActor` :!label _label)
    (elif (and _hasrocketlauncherbeenpickedup_ (< _returnvalue 6))
      (set `/Game/FirstPersonBP/AllAssets/Blueprints/FirstPersonCharacterBP.AmmoInRocketLauncherMag` 1 _asfirst_person_character_bp)
      (set `/Game/FirstPersonBP/AllAssets/Blueprints/FirstPersonCharacterBP.TotalRocketLauncherAmmo` 5 _asfirst_person_character_bp)
      (goto _label))))

(event `self.ReceiveTick`
  (params (DeltaSeconds :type "Float (single-precision)"))
  (`self.K2_AddActorLocalRotation` (struct :`Yaw` 3.0)))

(fn `UserConstructionScript`
  (set `ProjectileMovementComponent.InitialSpeed` (`self.ProjectileSpeed`) (`self.Projectile`)))