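; Robot damage projectile actor that hurts the first-person player character on contact.
; The construction script applies ProjectileSpeed as the projectile component's initial speed and redundantly assigns DamageDone to itself.
; Any overlap on the collision component destroys the actor, then subtracts DamageDone directly from CurrentHealth if the other actor is FirstPersonCharacterBP, bypassing Unreal's damage system.
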(event `self.CollisionComponent.OnComponentBeginOverlap`
  (params (OverlappedComponent :type "PrimitiveComponent Object Reference") (OtherActor :type "Actor Object Reference") (OtherComp :type "PrimitiveComponent Object Reference") (OtherBodyIndex :type Integer) (bFromSweep :type Boolean) (SweepResult :type "HitResult Structure (by ref)"))
  (`self.K2_DestroyActor`)
  (bind _asfirst_person_character_bp (cast `/Game/FirstPersonBP/AllAssets/Blueprints/FirstPersonCharacterBP` OtherActor))
  (set `/Game/FirstPersonBP/AllAssets/Blueprints/FirstPersonCharacterBP.CurrentHealth` (- (`/Game/FirstPersonBP/AllAssets/Blueprints/FirstPersonCharacterBP.CurrentHealth` _asfirst_person_character_bp) (`self.DamageDone`)) _asfirst_person_character_bp))

(fn `UserConstructionScript`
  (set `ProjectileMovementComponent.InitialSpeed` (`self.ProjectileSpeed`) (`self.Projectile`))
  (set `self.DamageDone` (`self.DamageDone`)))