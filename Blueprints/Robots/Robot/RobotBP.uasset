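; Enemy robot AI that patrols between two points until it sees the first-person player, then chases them with a walk animation.
; Tick polls health and capsule overlap, driving idle animation and a DoOnce-gated, cooldown-limited punch that spawns a RobotDamageBP at the overlapped actor.
; At zero health it plays a death sound, scatters randomized gibs, destroys itself and rolls rare speed or damage upgrade drops.
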(event `self.ReceiveBeginPlay`
  (`self.Patrol`))

(event `self.PawnSensing.OnSeePawn`
  (params (Pawn :type "Pawn Object Reference"))
  (set `self.InRange` true)
  (bind _asfirst_person_character_bp (cast `/Game/FirstPersonBP/AllAssets/Blueprints/FirstPersonCharacterBP` Pawn))
  (if (`self.PlayingAnim`)
    _
    (elif (not (`SkeletalMeshComponent.IsPlaying` (`self.SkeletalMesh`)))
      (`SkeletalMeshComponent.PlayAnimation` (`self.SkeletalMesh`) "/Game/FirstPersonBP/AllAssets/Animations/AnimationSequence/Robot_Animation_1_Anim_Armature_WalkCycle1.Robot_Animation_1_Anim_Armature_WalkCycle1" false)
      (set `self.PlayingAnim` true)))
  (`|AIMoveTo` self (0.0 0.0 0.0) _asfirst_person_character_bp
    (:`then`
      (`KismetSystemLibrary.Delay` 1.459)
      (set `self.PlayingAnim` false))))

(event `Patrol`
  (if (not (`self.InRange`))
    (`|AIMoveTo` self (0.0 0.0 0.0) (`self.Point 1`)
      (:`OnSuccess`
        (`KismetSystemLibrary.Delay` 3.0)
        (`|AIMoveTo` self (0.0 0.0 0.0) (`self.Point 2`)
          (:`then`
            (`KismetSystemLibrary.Delay` 3.0)
            (`self.Patrol`)))))))

(event `self.Capsule.OnComponentBeginOverlap`
  (params (OverlappedComponent :type "PrimitiveComponent Object Reference") (OtherActor :type "Actor Object Reference") (OtherComp :type "PrimitiveComponent Object Reference") (OtherBodyIndex :type Integer) (bFromSweep :type Boolean) (SweepResult :type "HitResult Structure (by ref)")))

(event `self.ReceiveTick`
  (params (DeltaSeconds :type "Float (single-precision)"))
  (bind _returnvalue (`KismetMathLibrary.RandomIntegerInRange` 0 31))
  (bind _returnvalue_2 (`self.GetTransform`))
  (bind (_x _y _z) (`KismetMathLibrary.GetAxes` (`self.GetControlRotation`)))
  (bind _returnvalue_3 (`KismetMathLibrary.MakeTransform` (`SceneComponent.K2_GetComponentLocation` (`self.Capsule`)) (`KismetMathLibrary.MakeRotFromX` (+ (+ _x (* _y (`KismetMathLibrary.RandomFloatInRange` -10.0 10.0))) (* _z (`KismetMathLibrary.RandomFloatInRange` -10.0 10.0))))))
  (if (<= (`self.RobotHealth`) 0.0)
    (`GameplayStatics.PlaySoundAtLocation` "/Game/FirstPersonBP/AllAssets/Sounds/RobotDeathSound.RobotDeathSound" (`self.K2_GetActorLocation`) :!label _label)
    (`|SpawnActorFromClass` "/Game/FirstPersonBP/AllAssets/Blueprints/Robots/Robot/RobotGib1.RobotGib1_C" _returnvalue_3 "Undefined" "OverrideRootScale" null (`KismetMathLibrary.RandomFloatInRange` 100.0 200.0))
    (`|SpawnActorFromClass` "/Game/FirstPersonBP/AllAssets/Blueprints/Robots/Robot/RobotGib1.RobotGib1_C" _returnvalue_3 "Undefined" "OverrideRootScale" null (`KismetMathLibrary.RandomFloatInRange` -100.0 -200.0))
    (`|SpawnActorFromClass` "/Game/FirstPersonBP/AllAssets/Blueprints/Robots/Robot/RobotGib2.RobotGib2_C" _returnvalue_3 "Undefined" "OverrideRootScale" null (`KismetMathLibrary.RandomFloatInRange` 100.0 -100.0))
    (`|SpawnActorFromClass` "/Game/FirstPersonBP/AllAssets/Blueprints/Robots/Robot/RobotGib3.RobotGib3_C" _returnvalue_3 "Undefined" "OverrideRootScale" null (`KismetMathLibrary.RandomFloatInRange` -100.0 -200.0))
    (`|SpawnActorFromClass` "/Game/FirstPersonBP/AllAssets/Blueprints/Robots/Robot/RobotGib4.RobotGib4_C" _returnvalue_3 "Undefined" "OverrideRootScale" null (`KismetMathLibrary.RandomFloatInRange` 100.0 200.0))
    (`self.K2_DestroyActor`)
    (if (== _returnvalue 17)
      _
      (elif (== _returnvalue 27)
        (`|SpawnActorFromClass` "/Game/FirstPersonBP/AllAssets/Blueprints/Powerups/SpeedUpgradeDropBP.SpeedUpgradeDropBP_C" _returnvalue_2 "Undefined" "OverrideRootScale")
        (goto _label_2 :!via `Reset`)
        (elif (== _returnvalue 29)
          (`|SpawnActorFromClass` "/Game/FirstPersonBP/AllAssets/Blueprints/Powerups/MoreDamageUpgradeDropBP.MoreDamageUpgradeDropBP_C" _returnvalue_2 "Undefined" "OverrideRootScale")
          (goto _label_2 :!via `Reset`))))
    (elif (`SkeletalMeshComponent.IsPlaying` (`self.SkeletalMesh`))
      (if (`PrimitiveComponent.IsOverlappingActor` (`self.Capsule`) (stale `self.Capsule.OnComponentBeginOverlap` OtherActor))
        (`/Engine/EditorBlueprintResources/StandardMacros.DoOnce` false :!label _label_2
          (:`Completed`
            (if (`self.CanFire?`)
              (set `self.CanFire?` false)
              (`SkeletalMeshComponent.PlayAnimation` (`self.SkeletalMesh`) "/Game/FirstPersonBP/AllAssets/Animations/AnimationSequence/Robot_Animation_1_Anim_Armature_Punch1.Robot_Animation_1_Anim_Armature_Punch1" false)
              (`KismetSystemLibrary.Delay` 0.39)
              (`|SpawnActorFromClass` "/Game/FirstPersonBP/AllAssets/Blueprints/Robots/Robot/RobotDamageBP.RobotDamageBP_C" (`KismetMathLibrary.Conv_VectorToTransform` (`self.K2_GetActorLocation` (stale `self.Capsule.OnComponentBeginOverlap` OtherActor))) "Undefined" "OverrideRootScale" null 99.0 1.0)
              (`KismetSystemLibrary.Delay` 1.61)
              (set `self.CanFire?` true)
              (if (<= (`self.RobotHealth`) 0.0) :!label _label_3
                (goto _label)
                (else
                  (goto _label_2 :!via `Reset`))))))
        (else
          (goto _label_3)))
      (elif (not (`self.Idle`))
        (set `self.Idle` true)
        (`SkeletalMeshComponent.PlayAnimation` (`self.SkeletalMesh`) "/Game/FirstPersonBP/AllAssets/Animations/AnimationSequence/Robot_Animation_1_Anim_Armature_Idle.Robot_Animation_1_Anim_Armature_Idle" false)
        (`KismetSystemLibrary.Delay` 1.21)
        (set `self.Idle` false)))))

(fn `UserConstructionScript`)