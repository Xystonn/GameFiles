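; BruteBP is a Brute robot enemy that turns toward and shoots at the player once its pawn sensing spots a pawn.
; Tick handles both yaw tracking of the living player and a DoOnce-gated firing loop that alternates BruteDamageBP projectiles from two sphere components on half-second delays.
; At zero health it plays a death sound, destroys itself and randomly rolls for a speed or damage upgrade drop.
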(event `self.ReceiveTick`
  (params (DeltaSeconds :type "Float (single-precision)"))
  (bind _returnvalue (`GameplayStatics.GetPlayerCharacter` 0))
  (bind _returnvalue_2 (`KismetMathLibrary.RandomIntegerInRange` 0 31))
  (bind _returnvalue_3 (`self.GetTransform`))
  (bind _hasbeenseen (`self.HasBeenSeen`))
  (bind (_x _y _z) (`KismetMathLibrary.GetAxes` (`self.GetControlRotation`)))
  (bind (_x_2 _y_2 _z_2) (`KismetMathLibrary.GetAxes` (`self.GetControlRotation`)))
  (if (<= (`self.BruteHealth`) 0.0)
    (`GameplayStatics.PlaySoundAtLocation` "/Game/FirstPersonBP/AllAssets/Sounds/RobotDeathSound.RobotDeathSound" (`self.K2_GetActorLocation`))
    (`self.K2_DestroyActor`)
    (if (== _returnvalue_2 17)
      _
      (elif (== _returnvalue_2 27)
        (`|SpawnActorFromClass` "/Game/FirstPersonBP/AllAssets/Blueprints/Powerups/SpeedUpgradeDropBP.SpeedUpgradeDropBP_C" _returnvalue_3 "Undefined" "OverrideRootScale")
        (goto _label :!via `Reset`)
        (elif (== _returnvalue_2 29)
          (`|SpawnActorFromClass` "/Game/FirstPersonBP/AllAssets/Blueprints/Powerups/MoreDamageUpgradeDropBP.MoreDamageUpgradeDropBP_C" _returnvalue_3 "Undefined" "OverrideRootScale")
          (goto _label :!via `Reset`))))
    (else
      (`|ExecutionSequence`
        (:`then_0`
          (if _hasbeenseen
            (bind _asfirst_person_character_bp (cast `/Game/FirstPersonBP/AllAssets/Blueprints/FirstPersonCharacterBP` _returnvalue))
            (if (not (`/Game/FirstPersonBP/AllAssets/Blueprints/FirstPersonCharacterBP.Dead` _asfirst_person_character_bp))
              (`SceneComponent.K2_SetWorldRotation` (`self.CapsuleComponent`) (`KismetMathLibrary.MakeRotator` 0.0 0.0 (.yaw (`KismetMathLibrary.FindLookAtRotation` (`self.K2_GetActorLocation`) (`self.K2_GetActorLocation` _returnvalue)))) false false))))
        (:`then_1`
          (if _hasbeenseen
            (`/Engine/EditorBlueprintResources/StandardMacros.DoOnce` false :!label _label
              (:`Completed`
                (if (`self.CanFire?`)
                  (set `self.CanFire?` false)
                  (`|SpawnActorFromClass` "/Game/FirstPersonBP/AllAssets/Blueprints/Robots/Brute/BruteDamageBP.BruteDamageBP_C" (`KismetMathLibrary.MakeTransform` (`SceneComponent.K2_GetComponentLocation` (`self.Sphere`)) (`KismetMathLibrary.MakeRotFromX` (+ (+ (+ _x (* _y (`KismetMathLibrary.RandomFloatInRange` 0.0 0.0))) (* _z (`KismetMathLibrary.RandomFloatInRange` 0.0 0.0))) (0.025 0.0 0.025)))) "Undefined" "OverrideRootScale" null 1000.0 0.8)
                  (`KismetSystemLibrary.Delay` 0.5)
                  (`|SpawnActorFromClass` "/Game/FirstPersonBP/AllAssets/Blueprints/Robots/Brute/BruteDamageBP.BruteDamageBP_C" (`KismetMathLibrary.MakeTransform` (`SceneComponent.K2_GetComponentLocation` (`self.Sphere3`)) (`KismetMathLibrary.MakeRotFromX` (+ (+ (+ _x_2 (* _y_2 (`KismetMathLibrary.RandomFloatInRange` 0.0 0.0))) (* _z_2 (`KismetMathLibrary.RandomFloatInRange` 0.0 0.0))) (0.025 0.0 0.025)))) "Undefined" "OverrideRootScale" null 1000.0 0.8)
                  (`KismetSystemLibrary.Delay` 0.5)
                  (set `self.CanFire?` true)
                  (goto _label :!via `Reset`))))))))))

(event `self.PawnSensing.OnSeePawn`
  (params (Pawn :type "Pawn Object Reference"))
  (set `self.HasBeenSeen` true))

(fn `UserConstructionScript`)