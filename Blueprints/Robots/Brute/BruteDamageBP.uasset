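; BruteDamageBP is a projectile, apparently for the Brute robot, that damages the first-person player character.
; Overlapping its collision component destroys it and, if the other actor is the player, subtracts DamageDone directly from CurrentHealth.
; A blocking hit spawns a plasma impact emitter, plus a short-lived rocket decal unless the surface is tagged NoDecal or Glass, and destroys it.
; The construction script applies ProjectileSpeed to the projectile's initial speed.
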(event `self.CollisionComponent.OnComponentBeginOverlap`
  (params (OverlappedComponent :type "PrimitiveComponent Object Reference") (OtherActor :type "Actor Object Reference") (OtherComp :type "PrimitiveComponent Object Reference") (OtherBodyIndex :type Integer) (bFromSweep :type Boolean) (SweepResult :type "HitResult Structure (by ref)"))
  (`self.K2_DestroyActor`)
  (bind _asfirst_person_character_bp (cast `/Game/FirstPersonBP/AllAssets/Blueprints/FirstPersonCharacterBP` OtherActor))
  (set `/Game/FirstPersonBP/AllAssets/Blueprints/FirstPersonCharacterBP.CurrentHealth` (- (`/Game/FirstPersonBP/AllAssets/Blueprints/FirstPersonCharacterBP.CurrentHealth` _asfirst_person_character_bp) (`self.DamageDone`)) _asfirst_person_character_bp))

(event `self.ReceiveHit`
  (params (MyComp :type "PrimitiveComponent Object Reference") (Other :type "Actor Object Reference") (OtherComp :type "PrimitiveComponent Object Reference") (bSelfMoved :type Boolean) (HitLocation :type "Vector Structure") (HitNormal :type "Vector Structure") (NormalImpulse :type "Vector Structure") (Hit :type "HitResult Structure (by ref)"))
  (bind _returnvalue (`KismetMathLibrary.Conv_VectorToRotator` HitNormal))
  (if (`self.ActorHasTag` Other "NoDecal")
    _
    (elif (not (`self.ActorHasTag` Other "Glass"))
      (`GameplayStatics.SpawnDecalAtLocation` "/Game/FirstPersonBP/AllAssets/Effects/Materials/Weapon/M_Rocket_Decal.M_Rocket_Decal" (16.0 32.0 32.0) HitLocation _returnvalue 10.0)))
  (`self.K2_DestroyActor`)
  (`GameplayStatics.SpawnEmitterAtLocation` "/Game/FirstPersonBP/AllAssets/ParticleEffects/PlasmaOrbHit.PlasmaOrbHit" HitLocation _returnvalue))

(fn `UserConstructionScript`
  (set `ProjectileMovementComponent.InitialSpeed` (`self.ProjectileSpeed`) (`self.Projectile`))
  (set `self.DamageDone` (`self.DamageDone`)))