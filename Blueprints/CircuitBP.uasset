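; Circuit box prop that reacts to being shot in two stages, destroying any actor that overlaps its Box trigger and counting each hit.
; The first hit, gated by a DoOnce, drops the lid with physics, disables Box1's collision, and removes the lid after a short delay.
; The second hit spawns three spark emitters in a short row just below the box's origin.
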(event `self.Box.OnComponentBeginOverlap`
  (params (OverlappedComponent :type "PrimitiveComponent Object Reference") (OtherActor :type "Actor Object Reference") (OtherComp :type "PrimitiveComponent Object Reference") (OtherBodyIndex :type Integer) (bFromSweep :type Boolean) (SweepResult :type "HitResult Structure (by ref)"))
  (bind _returnvalue (- (`SceneComponent.K2_GetComponentLocation` (`self.CircuitBox`)) (0.0 0.0 3.0)))
  (bind _returnvalue_2 (+ _returnvalue (-1.5 0.0 0.0)))
  (`self.K2_DestroyActor` OtherActor)
  (set `self.TimesShot` (+ (`self.TimesShot`) 1))
  (if (== (`self.TimesShot`) 2)
    (`GameplayStatics.SpawnEmitterAtLocation` "/Game/StarterContent/Particles/P_Sparks.P_Sparks" _returnvalue (struct))
    (`GameplayStatics.SpawnEmitterAtLocation` "/Game/StarterContent/Particles/P_Sparks.P_Sparks" _returnvalue_2)
    (`GameplayStatics.SpawnEmitterAtLocation` "/Game/StarterContent/Particles/P_Sparks.P_Sparks" (+ _returnvalue_2 (-1.5 0.0 0.0)))
    (else
      (`/Engine/EditorBlueprintResources/StandardMacros.DoOnce` false
        (:`Completed`
          (`PrimitiveComponent.SetSimulatePhysics` (`self.Lid`) true)
          (`PrimitiveComponent.SetCollisionEnabled` (`self.Box1`) "NoCollision")
          (`KismetSystemLibrary.Delay` 4.0)
          (`ActorComponent.K2_DestroyComponent` (`self.Lid`)))))))

(fn `UserConstructionScript`)