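; A damage upgrade pickup that temporarily sets the first-person character's DamageControlVariable flag.
; Box overlap with FirstPersonCharacterBP turns the flag on, then clears it after a fixed ten-second delay.
; Any actor overlap hides the skeletal mesh and disables box collision, leaving the actor alive rather than destroying it.
; Tick spins the actor by a fixed step each frame, independent of delta time.
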(event `self.ReceiveActorBeginOverlap`
  (params (OtherActor :type "Actor Object Reference"))
  (`SceneComponent.SetVisibility` (`self.SkeletalMesh`) false false)
  (`PrimitiveComponent.SetCollisionEnabled` (`self.Box`) "NoCollision"))

(event `self.Box.OnComponentBeginOverlap`
  (params (OverlappedComponent :type "PrimitiveComponent Object Reference") (OtherActor :type "Actor Object Reference") (OtherComp :type "PrimitiveComponent Object Reference") (OtherBodyIndex :type Integer) (bFromSweep :type Boolean) (SweepResult :type "HitResult Structure (by ref)"))
  (bind _asfirst_person_character_bp (cast `/Game/FirstPersonBP/AllAssets/Blueprints/FirstPersonCharacterBP` OtherActor))
  (set `/Game/FirstPersonBP/AllAssets/Blueprints/FirstPersonCharacterBP.DamageControlVariable` true _asfirst_person_character_bp)
  (`KismetSystemLibrary.Delay` 10.0)
  (set `/Game/FirstPersonBP/AllAssets/Blueprints/FirstPersonCharacterBP.DamageControlVariable` false _asfirst_person_character_bp))

(event `self.ReceiveTick`
  (params (DeltaSeconds :type "Float (single-precision)"))
  (`self.K2_AddActorLocalRotation` (struct :`Yaw` 3.0)))

(fn `UserConstructionScript`)