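; Rocket launcher projectile that explodes on hit and damages Robot and Brute enemies.
; Its construction script sets the projectile component's initial speed from a speed variable.
; On hit it spawns an explosion actor, leaves a temporary scorch decal unless the target is tagged NoDecal or Glass, and destroys itself.
; Damage is applied by casting the hit actor to each enemy type and directly subtracting a fixed amount from its health.
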(event `self.ReceiveHit`
  (params (MyComp :type "PrimitiveComponent Object Reference") (Other :type "Actor Object Reference") (OtherComp :type "PrimitiveComponent Object Reference") (bSelfMoved :type Boolean) (HitLocation :type "Vector Structure") (HitNormal :type "Vector Structure") (NormalImpulse :type "Vector Structure") (Hit :type "HitResult Structure (by ref)"))
  (`|SpawnActorFromClass` "/Game/FirstPersonBP/AllAssets/Blueprints/ExplosionBP.ExplosionBP_C" (`KismetMathLibrary.MakeTransform` HitLocation) "Undefined" "OverrideRootScale")
  (if (`self.ActorHasTag` Other "NoDecal")
    _
    (elif (not (`self.ActorHasTag` Other "Glass"))
      (`GameplayStatics.SpawnDecalAtLocation` "/Game/FirstPersonBP/AllAssets/Effects/Materials/Weapon/M_Rocket_Decal.M_Rocket_Decal" (20.0 40.0 40.0) HitLocation (`KismetMathLibrary.Conv_VectorToRotator` HitNormal) 10.0)))
  (`self.K2_DestroyActor`)
  (bind _asrobot_bp (cast `/Game/FirstPersonBP/AllAssets/Blueprints/Robots/Robot/RobotBP` Other)
    (:`then`
      (set `/Game/FirstPersonBP/AllAssets/Blueprints/Robots/Robot/RobotBP.RobotHealth` (- (`/Game/FirstPersonBP/AllAssets/Blueprints/Robots/Robot/RobotBP.RobotHealth` _asrobot_bp) 300.0) _asrobot_bp))
    (:`CastFailed`
      (bind _asbrute_bp (cast `/Game/FirstPersonBP/AllAssets/Blueprints/Robots/Brute/BruteBP` Other))
      (set `/Game/FirstPersonBP/AllAssets/Blueprints/Robots/Brute/BruteBP.BruteHealth` (- (`/Game/FirstPersonBP/AllAssets/Blueprints/Robots/Brute/BruteBP.BruteHealth` _asbrute_bp) 300.0) _asbrute_bp))))

(fn `UserConstructionScript`
  (set `ProjectileMovementComponent.InitialSpeed` (`self.ProjectileSpeed`) (`self.Projectile`)))